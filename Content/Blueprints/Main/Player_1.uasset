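; Player_1 is a player character Blueprint that provides movement, sprinting and a switch between first- and third-person views.
; Two identical movement functions store a vector and add it as CharacterMovement input, while Sprint toggles the maximum walk speed.
; SetView activates the chosen camera, deactivates the other and swaps visibility between first-person arms and body mesh.
; The event graph and construction script are empty, so all behavior lives in these callable functions.
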(event `self.ReceiveBeginPlay`)

(fn `Movement`
  (params (`Move Vector1` :type "Vector Structure"))
  (locals (`Move Vector` :type "Vector Structure" :default (0.0 0.0 0.0)))
  (set `local.Move Vector` `Move Vector1`)
  (`PawnMovementComponent.AddInputVector` (`self.CharacterMovement`) (`local.Move Vector`) false))

(fn `Movement_Side`
  (params (`Move Vector1` :type "Vector Structure"))
  (locals (`Move Vector` :type "Vector Structure" :default (0.0 0.0 0.0)))
  (set `local.Move Vector` `Move Vector1`)
  (`PawnMovementComponent.AddInputVector` (`self.CharacterMovement`) (`local.Move Vector`) false))

(fn `SetView`
  (params (FPC :type Boolean))
  (set `self.@FPC` FPC)
  (if (`self.@FPC`)
    (`ActorComponent.Activate` (`self.FirstPerson`) false)
    (`SceneComponent.SetVisibility` (`self.FirstPerson(arms)`) true false)
    (`SceneComponent.SetVisibility` (`self.Mesh`) false false)
    (`ActorComponent.Deactivate` (`self.ThirdPerson`))
    (else
      (`ActorComponent.Activate` (`self.ThirdPerson`) false)
      (`SceneComponent.SetVisibility` (`self.Mesh`) true false)
      (`SceneComponent.SetVisibility` (`self.FirstPerson(arms)`) false false)
      (`ActorComponent.Deactivate` (`self.FirstPerson`)))))

(fn `Sprint`
  (params (Sprint :type Boolean))
  (set `self.@sprint` Sprint)
  (if (`self.@sprint`)
    (set `CharacterMovementComponent.MaxWalkSpeed` 1000.0 (`self.CharacterMovement`))
    (else
      (set `CharacterMovementComponent.MaxWalkSpeed` 400.0 (`self.CharacterMovement`)))))

(fn `UserConstructionScript`)
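; MainPlayerController is the player controller that routes input to the controlled Player_1 pawn.
; BeginPlay caches the pawn and calls SetView(true), or prints an error if the cast fails.
; Movement axes pass scaled forward and right vectors to the pawn, while look axes drive controller pitch and yaw.
; Jump and view toggle act on press, and Sprint flips on both press and release, all without validity checks.
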(event `self.ReceiveBeginPlay`
  (bind _asplayer_1 (cast `/Game/Blueprints/Main/Player_1` (`self.K2_GetPawn`))
    (:`then`
      (set `self.My_pawn` _asplayer_1)
      (`/Game/Blueprints/Main/Player_1.SetView` (`self.My_pawn`) true))
    (:`CastFailed`
      (`KismetSystemLibrary.PrintString` "MainController Failedcast to pawn"))))

(event `InputAxis|Move Forward`
  (params (AxisValue :type "Float (single-precision)"))
  (if (`KismetSystemLibrary.IsValid` (`self.My_pawn`))
    (`/Game/Blueprints/Main/Player_1.Movement` (`self.My_pawn`) (* (`self.GetActorForwardVector` (`self.My_pawn`)) AxisValue))))

(event `InputAxis|Move Right`
  (params (AxisValue :type "Float (single-precision)"))
  (if (`KismetSystemLibrary.IsValid` (`self.My_pawn`))
    (`/Game/Blueprints/Main/Player_1.Movement_Side` (`self.My_pawn`) (* (`self.GetActorRightVector` (`self.My_pawn`)) AxisValue))))

(event `InputAxis|Look Up`
  (params (AxisValue :type "Float (single-precision)"))
  (`self.AddPitchInput` AxisValue))

(event `InputAxis|Turn around`
  (params (AxisValue :type "Float (single-precision)"))
  (`self.AddYawInput` AxisValue))

(event `InputAction|Jump`
  (params (Key :type "Key Structure"))
  (:`Pressed`
    (`Character.Jump` (`self.My_pawn`))))

(event `InputAction|SetView`
  (params (Key :type "Key Structure"))
  (bind _my_pawn (`self.My_pawn`))
  (:`Pressed`
    (`/Game/Blueprints/Main/Player_1.SetView` _my_pawn (not (`/Game/Blueprints/Main/Player_1.@FPC` _my_pawn)))))

(event `InputAction|Sprint`
  (params (Key :type "Key Structure"))
  (bind _my_pawn (`self.My_pawn`))
  (:`Pressed`
    (`/Game/Blueprints/Main/Player_1.Sprint` _my_pawn (not (`/Game/Blueprints/Main/Player_1.@sprint` _my_pawn)) :!label _label))
  (:`Released`
    (goto _label)))

(event `InputAction|Action`
  (params (Key :type "Key Structure")))

(event `InputAction|Fire`
  (params (Key :type "Key Structure")))

(fn `UserConstructionScript`)